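; Moving platform actor that travels in a loop through a list of editable PlatformPositions points.
; BeginPlay converts the local points to world space once, so the path stays fixed as the actor moves.
; Tick moves it toward the current target at Speed scaled by delta time, without sweep.
; Within a small distance of the target it advances the index, wrapping to the first point after the last.
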(event EventBeginPlay
  (for _array_element (Variables|Default|GetPlatformPositions)
    (Utilities|Array|Add (Variables|Default|GetWorldspacePositions) (Math|Transform|TransformLocation (Transformation|GetActorTransform) _array_element)))
  (Variables|Default|SetCurrentIndex 0))

(event EventTick
  (params (DeltaSeconds :type Float%20%28single-precision%29))
  (Variables|Default|SetTargetLocation (Utilities|Array|Get(acopy) (Variables|Default|GetWorldspacePositions) (Variables|Default|GetCurrentIndex)))
  (Variables|Default|SetCurrentLocation (Transformation|GetActorLocation))
  (Variables|Default|SetTargetDirection (- (Variables|Default|GetTargetLocation) (Variables|Default|GetCurrentLocation)))
  (Variables|Default|SetDistanceToMove (* (* (Math|Vector|Normalize (Variables|Default|GetTargetDirection)) (Variables|Default|GetSpeed)) (Utilities|Time|GetWorldDeltaSeconds)))
  (Transformation|SetActorLocation (+ (Transformation|GetActorLocation) (Variables|Default|GetDistanceToMove)) false false)
  (if (< (Math|Vector|VectorLength (- (Variables|Default|GetTargetLocation) (Variables|Default|GetCurrentLocation))) 1e+01)
    (if (== (Variables|Default|GetCurrentIndex) (Utilities|Array|LastIndex (Variables|Default|GetWorldspacePositions)))
      (Variables|Default|SetCurrentIndex 0)
      (else
        (Math|Integer|IncrementInt (Variables|Default|GetCurrentIndex))))))

(fn ConstructionScript)